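; BP_Door1 is a two-panel sliding door that opens only when every linked floor button matches its required state.
; On BeginPlay it caches both panels' closed positions and binds to the state-change dispatcher of each button in an array of button/state structs.
; Each change re-checks all pairs, then plays or reverses a Timeline that lerps the panels apart along local X.
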(event Custom|CustomEvent
  ;[0.15 0.15 0.15 0.5] Nos recorremos todos los botones para luego poder conectarnos al event dispacher de los botones. Ahora no son solo los botones, son los botones y el estado (struct)
  ;[0.15 0.15 0.15 0.5] Si todas están activados o no, ahora es que todo están en el estado correcto.
  (Variables|Default|SetareAllSameState true)
  (for _array_element (Variables|Default|Getbuttons)
    (if (not (== (.state _array_element) (Variables|/Game/00_Examen_UNIR/BP_FloorButton2.BP_FloorButton2_C|GetButtonActivated (.button _array_element))))
      (Variables|Default|SetareAllSameState false)))
  (if (Variables|Default|GetareAllSameState)
    ;;[0.15 0.15 0.15 0.5] Si se cumple se abren
    (CallFunction|OpenD true)
    (else
      ;[0.15 0.15 0.15 0.5] Si no se cumple se cierran
      (CallFunction|OpenD false))))

(event Custom|OpenD
  (params (open :type Boolean))
  ;[0.15 0.15 0.15 0.5] Evento que desplaza las puertas para que se abran
  (if open
    (bind _newtrack_0 (Timeline|Timeline Play)
      (:Update
        (Transformation|SetRelativeLocation (Variables|Default|GetRightDoor) (Math|Vector|Lerp(Vector) (Variables|Default|GetInitPos_RightDoor) (+ (Variables|Default|GetInitPos_RightDoor) "80.000000,0.000000,0.000000") _newtrack_0) false false)
        (Transformation|SetRelativeLocation (Variables|Default|GetLeftDoor) (Math|Vector|Lerp(Vector) (Variables|Default|GetInitPos_LeftDoor) (+ (Variables|Default|GetInitPos_LeftDoor) "-80.000000,0.000000,0.000000") _newtrack_0) false false)))
    (else
      (Timeline|Timeline Reverse))))

(event EventBeginPlay
  ;[0.15 0.15 0.15 0.5] Nos guardamos las posiciones iniciales de las puertas
  (Variables|Default|SetInitPos_RightDoor (Variables|/Script/Engine.SceneComponent|GetRelativeLocation (Variables|Default|GetRightDoor)))
  (Variables|Default|SetInitPos_LeftDoor (Variables|/Script/Engine.SceneComponent|GetRelativeLocation (Variables|Default|GetLeftDoor)))
  ;[0.15 0.15 0.15 0.5] Nos recorremos todos los botones para luego poder conectarnos al event dispacher de los botones. Ahora no son solo los botones, son los botones y el estado (struct)
  (for _array_element (Variables|Default|Getbuttons)
    (EventDispatchers|BindEventtoFloorButtonChangeState (.button _array_element) (delegate Custom|CustomEvent))))

(fn ConstructionScript)