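; Floor button that the third-person character toggles on and off with the E key while standing inside its box.
; Box overlap enables or disables keyboard input and swaps the outer ring material as a highlight.
; Each press swaps the hieroglyph's emissive material and fires CallDoorToOpen, which calls CallFloorButtonChangeState without forwarding the open state.
; A direct BPI_OpenDoor interface call to DoorActor remains as unconnected, never-run logic.
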(event OnComponentBeginOverlap(Box)
  (params (OverlappedComponent :type Primitive%20Component%20Object%20Reference) (OtherActor :type Actor%20Object%20Reference) (OtherComp :type Primitive%20Component%20Object%20Reference) (OtherBodyIndex :type Integer) (bFromSweep :type Boolean) (SweepResult :type Hit%20Result%20Structure%20%28by%20ref%29))
  ;[0.15 0.15 0.15 0.5] Ahora la condición de abrir o de enceder el botón, sea abierto o cerrado. La condición para poder abrir y cerrar es que esté dentro del box y que apriete la tecla E.
  (Utilities|Casting|CastToBP_ThirdPersonCharacter OtherActor)
  (Variables|Default|SetPlayerIsInside true)
  ;[0.15 0.15 0.15 0.5] Habilitamos el poder escuchar el teclado. Otra opcion es hacerlo con input actions.
  (Input|EnableInput (Game|GetPlayerController 0))
  ;[0.15 0.15 0.15 0.5] Hacemos que con el material cambiado parpadee cuando estamos dentro del boton
  (Rendering|Material|SetMaterial (Variables|Default|GetSM_circle_001) 1 "/Game/00_Examen_UNIR/M_Color1.M_Color1"))

(event OnComponentEndOverlap(Box)
  (params (OverlappedComponent :type Primitive%20Component%20Object%20Reference) (OtherActor :type Actor%20Object%20Reference) (OtherComp :type Primitive%20Component%20Object%20Reference) (OtherBodyIndex :type Integer))
  ;[0.15 0.15 0.15 0.5] Ahora la condición de abrir o de enceder el botón, sea abierto o cerrado. La condición para poder abrir y cerrar es que esté dentro del box y que apriete la tecla E.
  (Utilities|Casting|CastToBP_ThirdPersonCharacter OtherActor)
  (Variables|Default|SetPlayerIsInside false)
  (Input|DisableInput (Game|GetPlayerController 0))
  (Rendering|Material|SetMaterial (Variables|Default|GetSM_circle_001) 1 "/Game/LowPolyAssets/Materials/M_Color.M_Color"))

(event Custom|CallDoorToOpen
  (params (open :type Boolean))
  (Default|CallFloorButtonChangeState))

(event EventBeginPlay
  ;[0.15 0.15 0.15 0.5] Ponemos por defecto el material off (rojo) (puntitos del button)
  (Rendering|Material|SetMaterial (Variables|Default|GetSM_hieroglyph_007) 0 "/Game/00_Examen_UNIR/M_Emission_btn_Off.M_Emission_btn_Off")
  ;[0.15 0.15 0.15 0.5] Y también por defecto el que no parpadea (este en la parte de fuera del button)
  (Rendering|Material|SetMaterial (Variables|Default|GetSM_circle_001) 1 "/Game/LowPolyAssets/Materials/M_Color.M_Color"))

(event Collision|EventActorBeginOverlap
  (params (OtherActor :type Actor%20Object%20Reference)))

(event EventTick
  (params (DeltaSeconds :type Float%20%28single-precision%29)))

(event Input|KeyboardEvents|E
  (params (Key :type Key%20Structure :default "None"))
  ;[0.15 0.15 0.15 0.5] Una vez activado el input de teclado, queremos que esté dentro de lla box y que además tenga que apretar la E para abrir la puerta.
  (:Pressed
    (if (Variables|Default|GetPlayerIsInside)
      (bind _output_get (Variables|Default|SetButtonActivated (not (Variables|Default|GetButtonActivated))))
      (if _output_get
        (Rendering|Material|SetMaterial (Variables|Default|GetSM_hieroglyph_007) 0 "/Game/00_Examen_UNIR/M_Emission_btn_On.M_Emission_btn_On")
        (CallFunction|CallDoortoOpen true)
        (else
          (Rendering|Material|SetMaterial (Variables|Default|GetSM_hieroglyph_007) 0 "/Game/00_Examen_UNIR/M_Emission_btn_Off.M_Emission_btn_Off")
          (CallFunction|CallDoortoOpen false))))))

(fn ConstructionScript)